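; Player stats component that holds current and max HP and stamina for BP_ThirdPersonCharacter and mirrors them to its HUD widget.
; BeginPlay waits one tick so the HUD widget exists, then caches the owner and fills both bars and the HP text.
; Increase and decrease functions update the HUD directly; gains clamp to max, while decreases return true once the stat is depleted, without clamping at zero.
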(event EventBeginPlay
  ;[1 1 1] IDK What this is for exactly
  (Utilities|FlowControl|DelayUntilNextTick) ; HUD위젯 불러오기전에 뒤에 셋퍼센트가 먼저출력돼서 그거 방지용
  (bind _asbp_third_person_character (Utilities|Casting|CastToBP_ThirdPersonCharacter (Components|GetOwner)))
  (Variables|Default|SetPlayerCharacterBP _asbp_third_person_character)
  (Progress|SetPercent (Variables|/Game/UI/WB_HUD.WB_HUD_C|GetStaminaBar (Variables|/Game/ThirdPerson/Blueprints/BP_ThirdPersonCharacter.BP_ThirdPersonCharacter_C|GetHUD%20Widget (Variables|Default|GetPlayerCharacterBP))) (/ (Variables|Stamina|GetCurrentStamina) (Variables|Stamina|GetMaxStamina)))
  (Progress|SetPercent (Variables|/Game/UI/WB_HUD.WB_HUD_C|GetHPbar (Variables|/Game/ThirdPerson/Blueprints/BP_ThirdPersonCharacter.BP_ThirdPersonCharacter_C|GetHUD%20Widget (Variables|Default|GetPlayerCharacterBP))) (/ (Variables|Health|GetCurrentHP) (Variables|Health|GetMaxHP)))
  (Rendering|Components|TextRender|SetText (Variables|/Game/UI/WB_HUD.WB_HUD_C|GetHPValue (Variables|/Game/ThirdPerson/Blueprints/BP_ThirdPersonCharacter.BP_ThirdPersonCharacter_C|GetHUD%20Widget (Variables|Default|GetPlayerCharacterBP))) (Utilities|Text|ToText(Float) (Variables|Health|GetCurrentHP) "HalfToEven")))

(fn DecreaseHP
  (params (Damage :type Float%20%28double-precision%29))
  (bind _playercharacterbp (Variables|Default|GetPlayerCharacterBP))
  (bind _hud_widget (Variables|/Game/ThirdPerson/Blueprints/BP_ThirdPersonCharacter.BP_ThirdPersonCharacter_C|GetHUD%20Widget _playercharacterbp))
  (if (> (Variables|Health|GetCurrentHP) 0.0)
    (bind _output_get (Variables|Health|SetCurrentHP (- (Variables|Health|GetCurrentHP) Damage)))
    (Progress|SetPercent (Variables|/Game/UI/WB_HUD.WB_HUD_C|GetHPbar _hud_widget) (/ _output_get (Variables|Health|GetMaxHP)))
    (Rendering|Components|TextRender|SetText (Variables|/Game/UI/WB_HUD.WB_HUD_C|GetHPValue _hud_widget) (Utilities|Text|ToText(Float) (Variables|Health|GetCurrentHP) "HalfToEven"))
    (if (<= (Variables|Health|GetCurrentHP) 0.0)
      _
      (else
        (return false))))
  (return true))

(fn IncreaseMaxHP
  (params (HPIncremention :type Float%20%28double-precision%29))
  (bind _playercharacterbp (Variables|Default|GetPlayerCharacterBP))
  (bind _hud_widget (Variables|/Game/ThirdPerson/Blueprints/BP_ThirdPersonCharacter.BP_ThirdPersonCharacter_C|GetHUD%20Widget _playercharacterbp))
  (Variables|Health|SetMaxHP (+ (Variables|Health|GetMaxHP) HPIncremention))
  (Progress|SetPercent (Variables|/Game/UI/WB_HUD.WB_HUD_C|GetHPbar _hud_widget) (/ (Variables|Health|GetCurrentHP) (Variables|Health|GetMaxHP)))
  (Rendering|Components|TextRender|SetText (Variables|/Game/UI/WB_HUD.WB_HUD_C|GetHPValue _hud_widget) (Utilities|Text|ToText(Float) (Variables|Health|GetCurrentHP) "HalfToEven")))

(fn DecreaseStamina
  (params (Stamina%20Depleted :type Float%20%28double-precision%29))
  (if (> (Variables|Stamina|GetCurrentStamina) 0.0)
    (bind _output_get (Variables|Stamina|SetCurrentStamina (- (Variables|Stamina|GetCurrentStamina) Stamina%20Depleted)))
    (Progress|SetPercent (Variables|/Game/UI/WB_HUD.WB_HUD_C|GetStaminaBar (Variables|/Game/ThirdPerson/Blueprints/BP_ThirdPersonCharacter.BP_ThirdPersonCharacter_C|GetHUD%20Widget (Variables|Default|GetPlayerCharacterBP))) (/ _output_get (Variables|Stamina|GetMaxStamina)))
    (if (<= (Variables|Stamina|GetCurrentStamina) 0.0)
      _
      (else
        (return false))))
  (return true))

(fn IncreaseMaxStamina
  (params (StaminaIncremention :type Float%20%28double-precision%29))
  (Variables|Stamina|SetMaxStamina (+ (Variables|Stamina|GetMaxStamina) StaminaIncremention))
  (Progress|SetPercent (Variables|/Game/UI/WB_HUD.WB_HUD_C|GetStaminaBar (Variables|/Game/ThirdPerson/Blueprints/BP_ThirdPersonCharacter.BP_ThirdPersonCharacter_C|GetHUD%20Widget (Variables|Default|GetPlayerCharacterBP))) (/ (Variables|Stamina|GetCurrentStamina) (Variables|Stamina|GetMaxStamina))))

(fn IncreaseHP
  (params (AddedHP :type Float%20%28double-precision%29))
  (bind _playercharacterbp (Variables|Default|GetPlayerCharacterBP))
  (bind _hud_widget (Variables|/Game/ThirdPerson/Blueprints/BP_ThirdPersonCharacter.BP_ThirdPersonCharacter_C|GetHUD%20Widget _playercharacterbp))
  (Variables|Health|SetCurrentHP (+ (Variables|Health|GetCurrentHP) AddedHP))
  (if (> (Variables|Health|GetCurrentHP) (Variables|Health|GetMaxHP))
    (Variables|Health|SetCurrentHP (Variables|Health|GetMaxHP)))
  (Progress|SetPercent (Variables|/Game/UI/WB_HUD.WB_HUD_C|GetHPbar _hud_widget) (/ (Variables|Health|GetCurrentHP) (Variables|Health|GetMaxHP)))
  (Rendering|Components|TextRender|SetText (Variables|/Game/UI/WB_HUD.WB_HUD_C|GetHPValue _hud_widget) (Utilities|Text|ToText(Float) (Variables|Health|GetCurrentHP) "HalfToEven")))

(fn IncreaseStamina
  (params (AddedStamina :type Float%20%28double-precision%29))
  (Variables|Stamina|SetCurrentStamina (+ (Variables|Stamina|GetCurrentStamina) AddedStamina))
  (if (> (Variables|Stamina|GetCurrentStamina) (Variables|Stamina|GetMaxStamina))
    (Variables|Stamina|SetCurrentStamina (Variables|Stamina|GetMaxStamina)))
  (Progress|SetPercent (Variables|/Game/UI/WB_HUD.WB_HUD_C|GetStaminaBar (Variables|/Game/ThirdPerson/Blueprints/BP_ThirdPersonCharacter.BP_ThirdPersonCharacter_C|GetHUD%20Widget (Variables|Default|GetPlayerCharacterBP))) (/ (Variables|Stamina|GetCurrentStamina) (Variables|Stamina|GetMaxStamina))))